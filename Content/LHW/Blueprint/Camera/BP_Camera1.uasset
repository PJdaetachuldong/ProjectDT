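; BP_Camera1 is a camera Blueprint that turns to face the player pawn.
; On Tick it adds DeltaSeconds into a value of the same name and, only when that reaches a five-second threshold, sets the CameraComponent's world rotation with FindLookAtRotation.
; The rotation snaps directly to the pawn's location without interpolation.
; BeginPlay, overlap and construction logic are empty, and a leftover Delay node never runs.
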(event `self.ReceiveTick`
  (params (DeltaSeconds :type "Float (single-precision)"))
  (bind _output_get (set `self.Delta Seconds` (+ DeltaSeconds (`self.Delta Seconds`))))
  (if (>= _output_get 5.0)
    (`SceneComponent.K2_SetWorldRotation` (`self.CameraComponent`) (`KismetMathLibrary.FindLookAtRotation` (`SceneComponent.K2_GetComponentLocation` (`self.CameraComponent`)) (`self.K2_GetActorLocation` (`GameplayStatics.GetPlayerPawn` 0))) false false)))

(fn `UserConstructionScript`)